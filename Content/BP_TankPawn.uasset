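; BP_TankPawn is a tank pawn Blueprint that carries a progress bar widget component and a hotkey for a save test screen.
; Each tick it rotates the progress bar to face the player camera, billboard style.
; Pressing F5 creates a new WBP_SaveTest widget and adds it to the viewport, with no check for an existing one.
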(event Collision|EventActorBeginOverlap
  (params (OtherActor :type Actor%20Object%20Reference)))

(event EventTick
  (params (DeltaSeconds :type Float%20%28single-precision%29))
  (bind _progressbarwidgetcomponent (Variables|Default|GetProgressBarWidgetComponent))
  (Transformation|SetWorldRotation _progressbarwidgetcomponent (Math|Rotator|FindLookatRotation (Transformation|GetWorldLocation _progressbarwidgetcomponent) (Camera|GetCameraLocation (Game|GetPlayerCameraManager 0))) false false))

(event Input|KeyboardEvents|F5
  (params (Key :type Key%20Structure))
  (:Pressed
    (bind _returnvalue (UserInterface|CreateWidget "/Game/UI/WBP_SaveTest.WBP_SaveTest_C"))
    (UserInterface|Viewport|AddtoViewport _returnvalue 0)))

(fn ConstructionScript
  (|CallParentFunction))